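; Paper2D side-scroller enemy that patrols, chases the player and trades damage on contact.
; InterpToMovement patrols between two editable points, flipping the sprite on reverse, until left or right sensing overlaps start an AIMoveTo chase.
; Capsule overlaps with a player's sphere during a short glow pulse damage or, at zero health, destroy it; other player contact launches and hurts the player.
; Flipbook swaps, length-based delays and state flags gate these reactions.
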(event `self.InterpToMovement.OnInterpToReverse`
  (params (ImpactResult :type "HitResult Structure (by ref)") (Time :type "Float (single-precision)"))
  (bind _sprite (`self.Sprite`))
  ;[1 1 1] Turn around
  (`/Engine/EditorBlueprintResources/StandardMacros.FlipFlop`
    (:`A`
      (`SceneComponent.K2_SetWorldRotation` _sprite (struct :`Yaw` 180.0) false false)
      (set `self.MovingRight` true))
    (:`B`
      (`SceneComponent.K2_SetWorldRotation` :`self` _sprite)
      (set `self.MovingRight` false)))
  (`PaperFlipbookComponent.SetFlipbook` _sprite "/Game/Yugen/Assets/Flipbooks/Enemy/EnemyRun/Frames/enemyWalkAnim.enemyWalkAnim"))

(event `self.Capsule.OnComponentBeginOverlap`
  (params (OverlappedComponent :type "PrimitiveComponent Object Reference") (OtherActor :type "Actor Object Reference") (OtherComp :type "PrimitiveComponent Object Reference") (OtherBodyIndex :type Integer) (bFromSweep :type Boolean) (SweepResult :type "HitResult Structure (by ref)"))
  (bind _sprite (`self.Sprite`))
  (bind _sprite_2 (`self.Sprite`))
  (bind _interptomovement (`self.InterpToMovement`))
  ;[1 1 1] Collide with character
  ;[1 1 1] Collide with glow and die
  (cast `SphereComponent` OtherComp
    (:`then`
      (bind _asplayer_character (cast `/Game/Yugen/Blueprints/PlayerCharacter` OtherActor))
      (if (`/Game/Yugen/Blueprints/PlayerCharacter.GlowShortPulseActive` _asplayer_character)
        (if (> (`self.Enemy Health`) 0)
          (bind _flipbookalreadyenabled (`self.Compare Flipbook` self "/Game/Yugen/Assets/Flipbooks/Enemy/EnemyDamage/Frames/enemyDamage.enemyDamage"))
          (set `self.NotBeingDamaged` false)
          (if (not _flipbookalreadyenabled)
            (`InterpToMovementComponent.StopSimulating` _interptomovement SweepResult)
            (`self.Enemy Take Damage` self)
            (`NavMovementComponent.StopActiveMovement` (`self.CharacterMovement`))
            (`PaperFlipbookComponent.SetFlipbook` _sprite "/Game/Yugen/Assets/Flipbooks/Enemy/EnemyDamage/Frames/enemyDamage.enemyDamage")
            (`KismetSystemLibrary.Delay` (- (`PaperFlipbookComponent.GetFlipbookLength` _sprite) 3.0))
            (set `self.NotBeingDamaged` true)
            (`PaperFlipbookComponent.SetFlipbook` (`self.Sprite`) "/Game/Yugen/Assets/Flipbooks/Enemy/EnemyIdle/Frames/enemyIdle.enemyIdle"))
          (else
            (set `self.NotDying` false)
            (`InterpToMovementComponent.StopSimulating` _interptomovement SweepResult)
            (`self.SetActorEnableCollision` self false)
            (`NavMovementComponent.StopActiveMovement` (`self.CharacterMovement`))
            (`PaperFlipbookComponent.SetFlipbook` _sprite_2 "/Game/Yugen/Assets/Flipbooks/Enemy/EnemyDamage/Frames/enemyDamage.enemyDamage")
            (`KismetSystemLibrary.Delay` (- (`PaperFlipbookComponent.GetFlipbookLength` _sprite_2) 2.0))
            (`self.K2_DestroyActor` self)))))
    (:`CastFailed`
      (if (and (`self.NotDying`) (`self.NotBeingDamaged`))
        (bind _asplayer_character_2 (cast `/Game/Yugen/Blueprints/PlayerCharacter` OtherActor))
        (`self.LaunchCharacter` _asplayer_character_2 (`KismetMathLibrary.MakeVector` (* (.x (`.Normal` (`GameplayStatics.BreakHitResult` SweepResult))) -1500.0) 0.0 400.0) false false)
        (`PaperFlipbookComponent.SetFlipbook` (`self.Sprite`) "/Game/Yugen/Assets/Flipbooks/Enemy/EnemyAttack/Frames/enemyAttack.enemyAttack")
        (`/Game/Yugen/Blueprints/PlayerCharacter.TakeDamage` _asplayer_character_2)))))

(event `self.Sensing Right.OnComponentBeginOverlap`
  (params (OverlappedComponent :type "PrimitiveComponent Object Reference") (OtherActor :type "Actor Object Reference") (OtherComp :type "PrimitiveComponent Object Reference") (OtherBodyIndex :type Integer) (bFromSweep :type Boolean) (SweepResult :type "HitResult Structure (by ref)"))
  (bind _sprite (`self.Sprite`))
  ;[1 1 1] Chase Character
  (bind _output_get (set `self.Other Actor` OtherActor))
  (bind _aspaper_character (cast `PaperCharacter` _output_get))
  (cast `/Game/Yugen/Blueprints/PlayerCharacter` _aspaper_character)
  (if (and (`self.NotDying`) (`self.NotBeingDamaged`))
    (`SceneComponent.K2_SetWorldRotation` :`self` _sprite)
    (`PaperFlipbookComponent.SetFlipbook` _sprite "/Game/Yugen/Assets/Flipbooks/Enemy/EnemyWalk/Frames/enemyChase.enemyChase" :!label _label)
    (`InterpToMovementComponent.StopSimulating` (`self.InterpToMovement`) (`GameplayStatics.MakeHitResult` false))
    (`|AIMoveTo` self (0.0 0.0 0.0) (`self.Other Actor`) 0.0 true)))

(event `self.Sensing Left.OnComponentBeginOverlap`
  (params (OverlappedComponent :type "PrimitiveComponent Object Reference") (OtherActor :type "Actor Object Reference") (OtherComp :type "PrimitiveComponent Object Reference") (OtherBodyIndex :type Integer) (bFromSweep :type Boolean) (SweepResult :type "HitResult Structure (by ref)"))
  ;[1 1 1] Chase Character
  (bind _output_get (set `self.Other Actor` OtherActor))
  (bind _aspaper_character (cast `PaperCharacter` _output_get))
  (cast `/Game/Yugen/Blueprints/PlayerCharacter` _aspaper_character)
  (if (and (`self.NotDying`) (`self.NotBeingDamaged`))
    (`SceneComponent.K2_SetWorldRotation` (`self.Sprite`) (struct :`Yaw` 180.0) false false)
    (goto _label)))

(fn `Compare Flipbook`
  (params (Flipbook :type "PaperFlipbook Object Reference"))
  (returns (FlipbookAlreadyEnabled :type Boolean))
  (return (== Flipbook (`PaperFlipbookComponent.GetFlipbook` (`self.Sprite`)))))

(fn `Enemy Take Damage`
  (set `self.Enemy Health` (- (`self.Enemy Health`) 1)))

(fn `UserConstructionScript`
  (set `InterpToMovementComponent.ControlPoints` (`|MakeArray` (make `InterpControlPoint` (`self.PointA`)) (make `InterpControlPoint` (`self.PointB`))) (`self.InterpToMovement`)))