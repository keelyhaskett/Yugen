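; Puzzle door actor that is either open or closed, shown as a 2D sprite.
; Toggle, open, close and set-state functions only write the Open flag, leaving the decision of when to change it to callers.
; Open uses a RepNotify, whose handler swaps DoorSprite between the open and closed sprites so the visual follows the replicated state.
; The event graph and construction script are empty.
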(fn `OnRep_Open`
  (if (`self.Open`)
    (`PaperSpriteComponent.SetSprite` (`self.DoorSprite`) "/Game/Yugen/Assets/Sprites/DoorOpen.DoorOpen")
    (else
      (`PaperSpriteComponent.SetSprite` (`self.DoorSprite`) "/Game/Yugen/Assets/Sprites/DoorClosed.DoorClosed")))
  (return))

(fn `SetDoorClosed`
  (set `self.Open` false)
  (return))

(fn `SetDoorOpen`
  (set `self.Open` true)
  (return))

(fn `SetDoorState`
  (params (NewState :type Boolean))
  (returns (DoorState :type Boolean))
  (bind _output_get (set `self.Open` NewState))
  (return _output_get))

(fn `ToggleDoor`
  (returns (DoorState :type Boolean))
  (bind _output_get (set `self.Open` (not (`self.Open`))))
  (return _output_get))

(fn `UserConstructionScript`)