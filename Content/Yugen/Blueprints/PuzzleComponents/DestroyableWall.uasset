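; DestroyableWall is a puzzle component: a sprite wall that shows progressive cracking or breakage as it takes damage.
; An overlap from a PlayerCharacter adds one damage if that player's Glow is overlapping the wall, and helper functions set health or damage directly.
; Damage's RepNotify maps the rounded damage-to-health ratio onto eight sprites, from full to destroyed.
; Destruction only changes the sprite; collision and the actor are untouched.
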(event `self.ReceiveActorBeginOverlap`
  (params (OtherActor :type "Actor Object Reference"))
  (bind _asplayer_character (cast `/Game/Yugen/Blueprints/PlayerCharacter` OtherActor))
  (if (`PrimitiveComponent.IsOverlappingActor` (`/Game/Yugen/Blueprints/PlayerCharacter.Glow` _asplayer_character) self)
    (`self.IncrementDamage`)))

(fn `DestroyWall`
  (set `self.Damage` (`self.Health`))
  (return))

(fn `IncrementDamage`
  (returns (NewDamage :type Integer))
  (bind _output_get (set `self.Damage` (+ (`self.Damage`) 1)))
  (return _output_get))

(fn `IncrementDamageByAmount`
  (params (ChangeInDamage :type Integer))
  (returns (NewDamage :type Integer))
  (bind _output_get (set `self.Damage` (+ ChangeInDamage (`self.Damage`))))
  (return _output_get))

(fn `OnRep_Damage`
  (bind _returnvalue (`KismetMathLibrary.Round` (* (/ (`KismetMathLibrary.Conv_IntToDouble` (`self.Damage`)) (`KismetMathLibrary.Conv_IntToDouble` (`self.Health`))) 7.0)))
  (if (== _returnvalue 7)
    (`PaperSpriteComponent.SetSprite` (`self.Sprite`) "/Game/Yugen/Assets/Sprites/WallSprites/wallDestroyed_Sprite.wallDestroyed_Sprite")
    (elif (== _returnvalue 6)
      (`PaperSpriteComponent.SetSprite` (`self.Sprite`) "/Game/Yugen/Assets/Sprites/WallSprites/walls6hit_Sprite.walls6hit_Sprite")
      (elif (== _returnvalue 5)
        (`PaperSpriteComponent.SetSprite` (`self.Sprite`) "/Game/Yugen/Assets/Sprites/WallSprites/walls5hit_Sprite.walls5hit_Sprite")
        (elif (== _returnvalue 4)
          (`PaperSpriteComponent.SetSprite` (`self.Sprite`) "/Game/Yugen/Assets/Sprites/WallSprites/walls4hit_Sprite.walls4hit_Sprite")
          (elif (== _returnvalue 3)
            (`PaperSpriteComponent.SetSprite` (`self.Sprite`) "/Game/Yugen/Assets/Sprites/WallSprites/walls3hit_Sprite.walls3hit_Sprite")
            (elif (== _returnvalue 2)
              (`PaperSpriteComponent.SetSprite` (`self.Sprite`) "/Game/Yugen/Assets/Sprites/WallSprites/walls2hit_Sprite.walls2hit_Sprite")
              (elif (== _returnvalue 1)
                (`PaperSpriteComponent.SetSprite` (`self.Sprite`) "/Game/Yugen/Assets/Sprites/WallSprites/walls1hit_Sprite.walls1hit_Sprite")
                (elif (== _returnvalue 0)
                  (`PaperSpriteComponent.SetSprite` (`self.Sprite`) "/Game/Yugen/Assets/Sprites/WallSprites/wallFull_Sprite.wallFull_Sprite"))))))))))

(fn `SetWallDamage`
  (params (NewDamage :type Integer))
  (set `self.Damage` NewDamage)
  (return))

(fn `SetWallHealth`
  (params (NewHealth :type Integer))
  (set `self.Health` NewHealth)
  (return))

(fn `UserConstructionScript`)