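; Green crystal puzzle component that lights up when a player's active long-glow area overlaps it.
; Tick checks the PlayerCharacter's GlowLong overlap, then a DoOnce calls SetCrystalOn to set State and play a sound until ResetCrystalDoOnce re-arms it.
; OnRep_Open and UpdateFlipbookOnEnd drive the flipbook visuals from State, with functions to toggle, clear or set it directly.
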(event `self.ReceiveActorBeginOverlap`
  (params (OtherActor :type "Actor Object Reference")))

(event `ResetCrystalDoOnce`
  (goto _label :!via `Reset`))

(event `self.ReceiveTick`
  (params (DeltaSeconds :type "Float (single-precision)"))
  (bind _asplayer_character (cast `/Game/Yugen/Blueprints/PlayerCharacter` (stale `self.ReceiveActorBeginOverlap` OtherActor)))
  (if (and (`PrimitiveComponent.IsOverlappingActor` (`/Game/Yugen/Blueprints/PlayerCharacter.GlowLong` _asplayer_character) self) (`/Game/Yugen/Blueprints/PlayerCharacter.GlowLongActive` _asplayer_character))
    (`/Engine/EditorBlueprintResources/StandardMacros.DoOnce` false :!label _label
      (:`Completed`
        (`self.SetCrystalOn`)))))

(fn `OnRep_Open`
  (bind _flipbook (`self.Flipbook`))
  (if (`self.state`)
    (`PaperFlipbookComponent.SetLooping` _flipbook false)
    (`PaperFlipbookComponent.SetFlipbook` _flipbook "/Game/Yugen/Assets/Sprites/Puzzle/CrystalGreen/CrystalGreen1.CrystalGreen1")
    (else
      (`PaperFlipbookComponent.ReverseFromEnd` _flipbook)
      (`PaperFlipbookComponent.SetLooping` _flipbook false)
      (`PaperFlipbookComponent.SetFlipbook` _flipbook "/Game/Yugen/Assets/Sprites/Puzzle/CrystalGreen/CrystalGreen1.CrystalGreen1")))
  (return))

(fn `SetCrystalOff`
  (set `self.State` false)
  (return))

(fn `SetCrystalOn`
  (set `self.State` true)
  (`GameplayStatics.PlaySound2D` "/Game/Yugen/Assets/Sounds/green_crystal.green_crystal" 1.0 1.0 0.0 null null)
  (return))

(fn `SetCrystalState`
  (params (NewState :type Boolean))
  (set `self.State` NewState)
  (return))

(fn `ToggleCrystal`
  (returns (NewState :type Boolean))
  (bind _output_get (set `self.State` (not (`self.State`))))
  (return _output_get))

(fn `UpdateFlipbookOnEnd`
  (bind _flipbook (`self.Flipbook`))
  (if (`self.State`)
    (`PaperFlipbookComponent.SetFlipbook` _flipbook "/Game/Yugen/Assets/Sprites/Puzzle/CrystalGreen/CrystalGreen1.CrystalGreen1")
    (else
      (`PaperFlipbookComponent.SetFlipbook` _flipbook "/Game/Yugen/Assets/Sprites/Puzzle/CrystalGreen/CrystalGreenOff.CrystalGreenOff")))
  (return))

(fn `UserConstructionScript`)