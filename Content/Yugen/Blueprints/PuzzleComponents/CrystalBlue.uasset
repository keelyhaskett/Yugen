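; CrystalBlue is a puzzle-component door whose open state drives a blue Paper2D flipbook animation.
; Toggle and set functions change Open, and its OnRep plays the DoorBlue flipbook forward to open or in reverse to close.
; Closing binds a finished-playing event; OnFinishedClosing swaps in DoorGreenClosed, despite the blue naming, and unbinds it.
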(fn `OnFinishedClosing`
  (bind _breakingwall1 (`self.BreakingWall1`))
  (`PaperFlipbookComponent.SetFlipbook` _breakingwall1 "/Game/Yugen/Assets/Sprites/Puzzle/DoorGreen/DoorGreenClosed.DoorGreenClosed")
  (clear `PaperFlipbookComponent.OnFinishedPlaying` _breakingwall1)
  (return))

(fn `OnRep_Open`
  (bind _breakingwall1 (`self.BreakingWall1`))
  (if (`self.Open`)
    (`PaperFlipbookComponent.PlayFromStart` _breakingwall1)
    (`PaperFlipbookComponent.SetLooping` _breakingwall1 false)
    (`PaperFlipbookComponent.SetFlipbook` _breakingwall1 "/Game/Yugen/Assets/Sprites/Puzzle/DoorBlue/DoorBlue.DoorBlue")
    (else
      (add `PaperFlipbookComponent.OnFinishedPlaying` _breakingwall1 (`|CreateDelegate` :!event `OnFinishedClosing`))
      (`PaperFlipbookComponent.ReverseFromEnd` _breakingwall1)
      (`PaperFlipbookComponent.SetLooping` _breakingwall1 false)
      (`PaperFlipbookComponent.SetFlipbook` _breakingwall1 "/Game/Yugen/Assets/Sprites/Puzzle/DoorBlue/DoorBlue.DoorBlue")))
  (return))

(fn `SetDoorClosed`
  (set `self.Open` false)
  (return))

(fn `SetDoorOpen`
  (set `self.Open` true)
  (return))

(fn `SetDoorState`
  (params (NewState :type Boolean))
  (returns (DoorState :type Boolean))
  (if (!= NewState (`self.Open`))
    (bind _output_get (set `self.Open` NewState))
    (return _output_get)))

(fn `ToggleDoor`
  (returns (DoorState :type Boolean))
  (bind _output_get (set `self.Open` (not (`self.Open`))))
  (return _output_get))

(fn `UserConstructionScript`)