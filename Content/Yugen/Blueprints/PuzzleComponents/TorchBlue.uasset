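; Blue torch puzzle component that lights when a player character's active GlowLong overlaps it.
; Tick checks the glow overlap and fires a resettable DoOnce that turns the torch on.
; Setter and toggle functions change State, whose RepNotify plays the lighting flipbook once, calling Reverse when switching off.
; UpdateFlipbookOnEnd swaps in the matching on or off flipbook.
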(event `self.ReceiveActorBeginOverlap`
  (params (OtherActor :type "Actor Object Reference")))

(event `ResetTorchDoOnce`
  (goto _label :!via `Reset`))

(event `self.ReceiveTick`
  (params (DeltaSeconds :type "Float (single-precision)"))
  (bind _asplayer_character (cast `/Game/Yugen/Blueprints/PlayerCharacter` (stale `self.ReceiveActorBeginOverlap` OtherActor)))
  (if (and (`PrimitiveComponent.IsOverlappingActor` (`/Game/Yugen/Blueprints/PlayerCharacter.GlowLong` _asplayer_character) self) (`/Game/Yugen/Blueprints/PlayerCharacter.GlowLongActive` _asplayer_character))
    (`/Engine/EditorBlueprintResources/StandardMacros.DoOnce` false :!label _label
      (:`Completed`
        (`self.SetTorchOn`)))))

(fn `OnRep_State`
  (bind _paperflipbook (`self.PaperFlipbook`))
  (if (`self.State`)
    (`PaperFlipbookComponent.SetLooping` _paperflipbook false)
    (`PaperFlipbookComponent.SetFlipbook` _paperflipbook "/Game/Yugen/Assets/Sprites/Puzzle/LightBlue/LightBlue1.LightBlue1")
    (else
      (`PaperFlipbookComponent.Reverse` _paperflipbook)
      (`PaperFlipbookComponent.SetLooping` _paperflipbook false)
      (`PaperFlipbookComponent.SetFlipbook` _paperflipbook "/Game/Yugen/Assets/Sprites/Puzzle/LightBlue/LightBlue1.LightBlue1")))
  (return))

(fn `SetTorchOff`
  (set `self.State` false)
  (return))

(fn `SetTorchOn`
  (set `self.State` true)
  (return))

(fn `SetTorchState`
  (params (NewState :type Boolean))
  (set `self.State` NewState)
  (return))

(fn `ToggleTorch`
  (returns (NewState :type Boolean))
  (bind _output_get (set `self.State` (not (`self.State`))))
  (return _output_get))

(fn `UpdateFlipbookOnEnd`
  (bind _paperflipbook (`self.PaperFlipbook`))
  (if (`self.State`)
    (`PaperFlipbookComponent.SetFlipbook` _paperflipbook "/Game/Yugen/Assets/Sprites/Puzzle/LightBlue/LightBlueOn.LightBlueOn")
    (else
      (`PaperFlipbookComponent.SetFlipbook` _paperflipbook "/Game/Yugen/Assets/Sprites/Puzzle/LightBlue/LightBlueOff.LightBlueOff")))
  (return))

(fn `UserConstructionScript`)