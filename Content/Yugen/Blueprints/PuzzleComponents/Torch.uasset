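; Torch puzzle switch that toggles on or off when a PlayerCharacter begins overlapping it while that character's Glow also overlaps it.
; Toggle and set functions write a boolean State, whose RepNotify swaps the lit or unlit sprite on LeverSprite.
; The notify then fires ValueUpdated with SetSprite's return value rather than State, and that event relays through CallValueUpdatedEvent.
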(event `self.ReceiveActorBeginOverlap`
  (params (OtherActor :type "Actor Object Reference"))
  (bind _asplayer_character (cast `/Game/Yugen/Blueprints/PlayerCharacter` OtherActor))
  (if (`PrimitiveComponent.IsOverlappingActor` (`/Game/Yugen/Blueprints/PlayerCharacter.Glow` _asplayer_character) self)
    (`self.ToggleSwitch`)))

(event `ValueUpdated`
  (params (NewState :type Boolean))
  (`self.ValueUpdatedEvent`))

(fn `OnRep_State`
  (if (`self.State`)
    (bind _returnvalue (`PaperSpriteComponent.SetSprite` (`self.LeverSprite`) "/Game/Yugen/Assets/Sprites/torchOn_Sprite.torchOn_Sprite"))
    (`self.ValueUpdated` _returnvalue)
    (else
      (bind _returnvalue_2 (`PaperSpriteComponent.SetSprite` (`self.LeverSprite`) "/Game/Yugen/Assets/Sprites/torchOff_Sprite.torchOff_Sprite"))
      (`self.ValueUpdated` _returnvalue_2)))
  (return))

(fn `SetSwitchOff`
  (set `self.State` false)
  (return))

(fn `SetSwitchOn`
  (set `self.State` true)
  (return))

(fn `SetSwitchState`
  (params (NewState :type Boolean))
  (set `self.State` NewState)
  (return))

(fn `ToggleSwitch`
  (returns (NewState :type Boolean))
  (bind _output_get (set `self.State` (not (`self.State`))))
  (return _output_get))

(fn `UserConstructionScript`)