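; Crisis boss enemy that chases the player, attacks on contact and can be destroyed by the player's glow pulse.
; Tick moves it toward the player via AIMoveTo, while capsule overlap attempts a back-step (noted as broken), then deals damage and starts a cooldown.
; During cooldown, sphere overlaps with an active short pulse reduce its health, or destroy it once health is depleted.
; Flipbook comparisons double as state guards.
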(event `self.Capsule.OnComponentBeginOverlap`
  (params (OverlappedComponent :type "PrimitiveComponent Object Reference") (OtherActor :type "Actor Object Reference") (OtherComp :type "PrimitiveComponent Object Reference") (OtherBodyIndex :type Integer) (bFromSweep :type Boolean) (SweepResult :type "HitResult Structure (by ref)"))
  (bind _sprite (`self.Sprite`))
  (bind (_returnvalue_x _returnvalue_y _returnvalue_z) (`KismetMathLibrary.BreakVector` (`self.K2_GetActorLocation` self)))
  (bind _returnvalue (`PaperFlipbookComponent.GetFlipbookLength` _sprite))
  ;[1 1 1] Collide with character
  (`PaperFlipbookComponent.SetFlipbook` (`self.Sprite`) "/Game/Yugen/Assets/Flipbooks/Boss/Crisis/Idle/Frames/CrisisIdle.CrisisIdle") ; Sets to idle in case it is colliding with something that it won't attack
  (if (and (`self.NotCooldown`) (`self.NotDying`))
    (bind _asplayer_character (cast `/Game/Yugen/Blueprints/PlayerCharacter` OtherActor))
    (`|AIMoveTo` self (`KismetMathLibrary.MakeVector` (- _returnvalue_x 100.0) _returnvalue_y _returnvalue_z) null 100.0
      (:`then`
        (`PaperFlipbookComponent.SetFlipbook` (`self.Sprite`) "/Game/Yugen/Assets/Flipbooks/Boss/Crisis/Attack/Frames/CrisisAttack.CrisisAttack")
        (`/Game/Yugen/Blueprints/PlayerCharacter.TakeDamage` _asplayer_character)
        (`KismetSystemLibrary.Delay` (`PaperFlipbookComponent.GetFlipbookLength` (`self.Sprite`)))
        (set `self.NotCooldown` false)
        (`PaperFlipbookComponent.SetFlipbook` (`self.Sprite`) "/Game/Yugen/Assets/Flipbooks/Boss/Crisis/Idle/Frames/CrisisIdle.CrisisIdle")
        (`KismetSystemLibrary.Delay` 5.0)
        (set `self.NotCooldown` true)))
    (elif (and (not (`self.NotCooldown`)) (`self.NotDying`))
      (cast `SphereComponent` OtherComp)
      (bind _asplayer_character_2 (cast `/Game/Yugen/Blueprints/PlayerCharacter` OtherActor))
      ;[1 1 1] Take damage and die
      (if (`/Game/Yugen/Blueprints/PlayerCharacter.GlowShortPulseActive` _asplayer_character_2)
        (if (> (`self.Crisis Health`) 0)
          (bind _flipbookalreadyenabled (`self.Compare Flipbook` self "/Game/Yugen/Assets/Flipbooks/Boss/Crisis/Damage/Frames/CrisisDamage.CrisisDamage"))
          (if (not _flipbookalreadyenabled)
            (`PaperFlipbookComponent.SetFlipbook` _sprite "/Game/Yugen/Assets/Flipbooks/Boss/Crisis/Damage/Frames/CrisisDamage.CrisisDamage")
            (`KismetSystemLibrary.Delay` _returnvalue)
            (`self.Crisis Take Damage` self)
            (`PaperFlipbookComponent.SetFlipbook` _sprite "/Game/Yugen/Assets/Flipbooks/Boss/Crisis/Idle/Frames/CrisisIdle.CrisisIdle"))
          (else
            (bind _flipbookalreadyenabled_2 (`self.Compare Flipbook` self null))
            (if (not _flipbookalreadyenabled_2)
              (`PaperFlipbookComponent.SetFlipbook` _sprite null)
              (set `self.NotDying` false)
              (`KismetSystemLibrary.Delay` _returnvalue)
              (`self.K2_DestroyActor` self))))))))

(event `self.ReceiveTick`
  (params (DeltaSeconds :type "Float (single-precision)"))
  ;[1 1 1] Chase character
  (bind _flipbookalreadyenabled (`self.Compare Flipbook` self "/Game/Yugen/Assets/Flipbooks/Boss/Crisis/Attack/Frames/CrisisAttack.CrisisAttack"))
  (if _flipbookalreadyenabled
    _
    (elif (and (`self.NotCooldown`) (`self.NotDying`))
      (`PaperFlipbookComponent.SetFlipbook` (`self.Sprite`) "/Game/Yugen/Assets/Flipbooks/Boss/Crisis/Walk/Frames/CrisisWalk.CrisisWalk")
      (bind _movementresult (`|AIMoveTo` self (0.0 0.0 0.0) (`GameplayStatics.GetPlayerCharacter` 0) 100.0 true)
        (:`then`
          (`KismetSystemLibrary.PrintString` (`|GetEnumeratorNameAsString` _movementresult)))))))

(fn `Compare Flipbook`
  (params (Flipbook :type "PaperFlipbook Object Reference"))
  (returns (FlipbookAlreadyEnabled :type Boolean))
  (return (== Flipbook (`PaperFlipbookComponent.GetFlipbook` (`self.Sprite`)))))

(fn `Crisis Take Damage`
  ;[0.474 0 0.03306] Take damage
  (set `self.Crisis Health` (- (`self.Crisis Health`) 1)))

(fn `UserConstructionScript`)