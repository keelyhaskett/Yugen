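; Boss actor that moves along a three-point path and hurts the player on contact.
; The construction script feeds the PointA, PointB and PointC variables into InterpToMovement as relative control points.
; When the Box overlaps a PlayerCharacter, it launches the player along X, scaled by the sweep normal, with a slight upward kick, then calls TakeDamage on them.
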(event `self.Box.OnComponentBeginOverlap`
  (params (OverlappedComponent :type "PrimitiveComponent Object Reference") (OtherActor :type "Actor Object Reference") (OtherComp :type "PrimitiveComponent Object Reference") (OtherBodyIndex :type Integer) (bFromSweep :type Boolean) (SweepResult :type "HitResult Structure (by ref)"))
  ;[1 1 1] Collide with character
  (bind _asplayer_character (cast `/Game/Yugen/Blueprints/PlayerCharacter` OtherActor))
  (`self.LaunchCharacter` _asplayer_character (`KismetMathLibrary.MakeVector` (* (.x (`.Normal` (`GameplayStatics.BreakHitResult` SweepResult))) -1500.0) 0.0 200.0) false false)
  (`/Game/Yugen/Blueprints/PlayerCharacter.TakeDamage` _asplayer_character))

(fn `UserConstructionScript`
  (set `InterpToMovementComponent.ControlPoints` (`|MakeArray` (make `InterpControlPoint` (`self.Point A`)) (make `InterpControlPoint` (`self.Point B`)) (make `InterpControlPoint` (`self.Point C`))) (`self.InterpToMovement`)))