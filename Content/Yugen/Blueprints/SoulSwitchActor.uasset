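; Controllable soul pawn that moves in the X/Z plane and transfers player control to a PlayerCharacter it touches.
; Movement input works while it is within a set maximum distance of the initial character, otherwise it is forced back toward that character.
; On overlapping a character's capsule, it briefly ignores move input while blending the camera to that character, then possesses it and destroys itself.
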(event `self.ReceiveActorBeginOverlap`
  (params (OtherActor :type "Actor Object Reference"))
  (bind _returnvalue (`GameplayStatics.GetPlayerController` 0))
  (bind _asplayer_character (cast `/Game/Yugen/Blueprints/PlayerCharacter` OtherActor))
  (if (`PrimitiveComponent.IsOverlappingActor` (`Character.CapsuleComponent` _asplayer_character) self)
    (`Controller.SetIgnoreMoveInput` _returnvalue true)
    (`PlayerController.SetViewTargetWithBlend` _returnvalue _asplayer_character 0.2 "VTBlend_Linear" 0.2 false)
    (`KismetSystemLibrary.Delay` 0.2)
    (`Controller.SetIgnoreMoveInput` _returnvalue false)
    (`Controller.Possess` _returnvalue _asplayer_character)
    (`self.K2_DestroyActor`)))

(event `InputAxis|MoveRight`
  (params (AxisValue :type "Float (single-precision)"))
  ;[1 1 1] Handle movement
  (if (> AxisValue 0.0)
    _
    (elif (< AxisValue 0.0)
      _
      (else
        _)))
  (bind _isatmaxdistance (`self.IsAtMax`))
  (if _isatmaxdistance
    (`self.AddMovementInput` (1.0 0.0 0.0) AxisValue)
    (else
      (`self.AddMovementInput` (`KismetMathLibrary.GetDirectionUnitVector` (`self.K2_GetActorLocation`) (`self.K2_GetActorLocation` (`self.InitalCharacter`))) 1.0 true :!label _label)
      (`KismetSystemLibrary.Delay` 0.2))))

(event `InputAxis|MoveUp`
  (params (AxisValue :type "Float (single-precision)"))
  ;[1 1 1] Handle movement
  (if (> AxisValue 0.0)
    _
    (elif (< AxisValue 0.0)
      _
      (else
        _)))
  (bind _isatmaxdistance (`self.IsAtMax`))
  (if _isatmaxdistance
    (`self.AddMovementInput` (0.0 0.0 1.0) AxisValue)
    (else
      (goto _label))))

(fn `IsAtMax`
  (returns (IsAtMaxDistance :type Boolean))
  (return (<= (`KismetMathLibrary.Sqrt` (+ (`KismetMathLibrary.Square` (- (.z (`self.K2_GetActorLocation` (`self.InitalCharacter`))) (.z (`self.K2_GetActorLocation`)))) (`KismetMathLibrary.Square` (- (.x (`self.K2_GetActorLocation` (`self.InitalCharacter`))) (.x (`self.K2_GetActorLocation`)))))) (`self.MaxDistance`))))

(fn `SetInitalCharacter`
  (params (NewParam :type "Actor Object Reference"))
  (set `self.InitalCharacter` NewParam)
  (return))

(fn `SetMaxDistance`
  (params (NewDistance :type "Float (double-precision)"))
  (set `self.MaxDistance` NewDistance)
  (return))

(fn `UserConstructionScript`)