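; Player character Yugen for a 2D side-scroller, with movement, jumping and velocity-driven flipbook selection.
; Three glow abilities (short pulse, long pulse, long glow) each spend their own health, spawn a Glow actor and scale up sphere components on Tick.
; Frame-counted recharges run one at a time in priority order; death requires all three healths at zero.
; Soul Swap spawns a SoulSwitchActor ahead, blends the camera to it, then possesses it.
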(event `InputAction|ExpandLongGlow`
  (params (Key :type "Key Structure"))
  (bind _returnvalue (`SceneComponent.K2_GetComponentToWorld` (`self.CapsuleComponent`)))
  ;[1 1 1] Enable Glow
  (:`Pressed`
    (bind (_canuseshortpulse _canuselongpulse _canuselongglow) (`self.CanUseGlow` false false true))
    (if _canuselongglow
      (set `self.GlowLongActive` _canuselongglow)
      (bind _endhealth (`self.ProcessGlowDamage` (`self.LongHealth`)))
      (set `self.LongHealth` _endhealth)
      (bind _returnvalue_2 (`|SpawnActorFromClass` "/Game/Yugen/Blueprints/GlowComponents/Glow.Glow_C" (`KismetMathLibrary.MakeTransform` (`KismetMathLibrary.MakeVector` (.x (.location _returnvalue)) (+ (.y (.location _returnvalue)) 5.0) (.z (.location _returnvalue))) (.rotation _returnvalue) (.scale _returnvalue)) "Undefined" "OverrideRootScale" null null :!label _label))
      (set `self.CurrentGlow` _returnvalue_2)))
  (:`Released`
    (set `self.GlowLongActive` false)
    (set `self.GlowLongCharged` false)))

(event `InputAction|SoulSwap`
  (params (Key :type "Key Structure"))
  (bind _returnvalue (`GameplayStatics.GetPlayerController` 0))
  (bind _returnvalue_2 (`GameplayStatics.GetPlayerController` 0))
  ;[1 1 1] Soul Swap - Spawns new actor and swaps the controller
  (:`Pressed`
    (if (`self.Dead`)
      _
      (elif (`self.isMovingRight`)
        (bind _returnvalue_3 (`|SpawnActorFromClass` "/Game/Yugen/Blueprints/SoulSwitchActor.SoulSwitchActor_C" (`KismetMathLibrary.MakeTransform` (`KismetMathLibrary.MakeVector` (+ (.x (.location (`self.GetTransform` self))) 150.0) (.y (.location (`self.GetTransform` self))) (.z (.location (`self.GetTransform` self)))) (.rotation (`self.GetTransform` self)) (.scale (`self.GetTransform` self))) "AlwaysSpawn" "OverrideRootScale" null null))
        (`/Game/Yugen/Blueprints/SoulSwitchActor.SetInitalCharacter` _returnvalue_3 self)
        (`Controller.SetIgnoreMoveInput` _returnvalue true)
        (`PlayerController.SetViewTargetWithBlend` _returnvalue _returnvalue_3 0.2 "VTBlend_Linear" 0.2 false)
        (`KismetSystemLibrary.Delay` 0.2)
        (`Controller.SetIgnoreMoveInput` _returnvalue false)
        (`Controller.Possess` _returnvalue _returnvalue_3)
        (else
          (bind _returnvalue_4 (`|SpawnActorFromClass` "/Game/Yugen/Blueprints/SoulSwitchActor.SoulSwitchActor_C" (`KismetMathLibrary.MakeTransform` (`KismetMathLibrary.MakeVector` (+ (.x (.location (`self.GetTransform` self))) -150.0) (.y (.location (`self.GetTransform` self))) (.z (.location (`self.GetTransform` self)))) (.rotation (`self.GetTransform` self)) (.scale (`self.GetTransform` self))) "AlwaysSpawn" "OverrideRootScale" null null))
          (`/Game/Yugen/Blueprints/SoulSwitchActor.SetInitalCharacter` _returnvalue_4 self)
          (`Controller.SetIgnoreMoveInput` _returnvalue_2 true)
          (`PlayerController.SetViewTargetWithBlend` _returnvalue_2 _returnvalue_4 0.2 "VTBlend_Linear" 0.2 false)
          (`KismetSystemLibrary.Delay` 0.2)
          (`Controller.SetIgnoreMoveInput` _returnvalue_2 false)
          (`Controller.Possess` _returnvalue_2 _returnvalue_4))))))

(event `InputAction|ExpandLongPulseGlow`
  (params (Key :type "Key Structure"))
  ;[1 1 1] Enable Glow
  (:`Pressed`
    (bind (_canuseshortpulse _canuselongpulse) (`self.CanUseGlow` false true))
    (if _canuselongpulse
      (set `self.GlowLongPulseActive` _canuselongpulse)
      (bind _endhealth (`self.ProcessGlowDamage` (`self.LongPulseHealth`)))
      (set `self.LongPulseHealth` _endhealth)
      (goto _label)))
  (:`Released`
    (set `self.GlowLongPulseActive` false)
    (set `self.GlowLongPulseCharged` false)))

(event `InputAction|ExpandShortPulseGlow`
  (params (Key :type "Key Structure"))
  ;[1 1 1] Enable Glow
  (:`Pressed`
    (bind _canuseshortpulse (`self.CanUseGlow` true))
    (if _canuseshortpulse
      (set `self.GlowShortPulseActive` _canuseshortpulse)
      (bind _endhealth (`self.ProcessGlowDamage` (`self.ShortPulseHealth`)))
      (set `self.ShortPulseHealth` _endhealth)
      (goto _label)))
  (:`Released`
    (set `self.GlowShortPulseActive` false)
    (set `self.GlowShortPulseCharged` false)))

(event `InputAction|Jump`
  (params (Key :type "Key Structure"))
  (bind _dead (`self.Dead`))
  ;[1 1 1] Handle Jump
  (:`Pressed`
    (if (not _dead) :!label _label_2
      (`self.Jump`)))
  (:`Released`
    (if (not _dead) :!label _label_3
      (`self.StopJumping`))))

(event `self.ReceiveBeginPlay`
  (bind _springarm (`self.SpringArm`))
  (bind _springarm_2 (`self.SpringArm`))
  ;[1 1 1] Start Game
  (`ActorComponent.SetIsReplicated` (`self.Sprite`) true)
  ;[1 1 1] Create health widget (for testing)
  (bind _returnvalue (`|CreateWidget` "/Game/Yugen/Blueprints/HealthHUD.HealthHUD_C"))
  (`UserWidget.AddToViewport` _returnvalue 0)
  ;[1 1 1] Set Initial Values
  (set `self.ShortPulseHealth` 10)
  (set `self.LongPulseHealth` 10)
  (set `self.LongHealth` 10)
  (bind _returnvalue_2 (`GameplayStatics.GetCurrentLevelName` true))
  (`|ExecutionSequence`
    (:`then_0`
      (if (`KismetStringLibrary.Contains` _returnvalue_2 "Boss")
        (set `SpringArmComponent.TargetArmLength` 200000.0 _springarm_2)
        (else
          (set `SpringArmComponent.TargetArmLength` 100000.0 _springarm_2))))
    (:`then_1`
      (if true
        (set `SpringArmComponent.CameraLagSpeed` 2.0 _springarm)
        (else
          (set `SpringArmComponent.CameraLagSpeed` 5.0 _springarm))))))

(event `InputTouch`
  (params (Location :type "Vector Structure") (FingerIndex :type "ETouchIndex Enum"))
  ;[1 1 1] Handle Jump
  (:`Pressed`
    (goto _label_2))
  (:`Released`
    (goto _label_3)))

(event `self.ReceiveTick`
  (params (DeltaSeconds :type "Float (single-precision)"))
  (bind _returnvalue (`self.GetController`))
  (bind _returnvalue_2 (`self.GetController`))
  (bind _glowlongactive (`self.GlowLongActive`))
  (bind _glowlongpulseactive (`self.GlowLongPulseActive`))
  (bind _glowshortpulseactive (`self.GlowShortPulseActive`))
  (`|ExecutionSequence`
    (:`then_0`
      ;[1 1 1] Grow Glow
      (if (`self.Dead`)
        _
        (elif _glowshortpulseactive
          (`self.ExpandGlow` (`self.GlowShortPulse`) _glowshortpulseactive)
          (elif _glowlongpulseactive
            (`self.ExpandGlow` (`self.GlowLongPulse`) false _glowlongpulseactive)
            (elif _glowlongactive
              (set `self.GlowLongStarted` true)
              (`self.ExpandGlow` (`self.GlowLong`) false false _glowlongactive)
              (elif (`self.GlowFinished`)
                (`self.ResetGlow` (`self.GlowLong`))
                (`self.ResetGlow` (`self.GlowLongPulse`))
                (`self.ResetGlow` (`self.GlowShortPulse`))
                (bind _outactors (`GameplayStatics.GetAllActorsOfClass` "/Game/Yugen/Blueprints/PuzzleComponents/Torch.Torch_C"))
                (for _array_element _outactors
                  (`/Game/Yugen/Blueprints/PuzzleComponents/Torch.ResetTorchDoOnce` _array_element))))))))
    (:`then_1`
      ;[1 1 1] Tick - Updates animation
      (`self.ChangeFlipBook` null)
      (`self.UpdateAnimation`)
      (`/Engine/EditorBlueprintResources/StandardMacros.CompareFloat` (.x (`MovementComponent.Velocity` (`self.GetMovementComponent`)))
        (:`>`
          (`/Engine/EditorBlueprintResources/StandardMacros.IsValid` _returnvalue_2 :!label _label_4
            (:`Is Valid`
              (`Controller.SetControlRotation` _returnvalue_2 (`KismetMathLibrary.MakeRotator` 0.0)))))
        (:`==`
          (if (`self.isMovingRight`)
            (goto _label_4)
            (else
              (`/Engine/EditorBlueprintResources/StandardMacros.IsValid` _returnvalue :!label _label_5
                (:`Is Valid`
                  (`Controller.SetControlRotation` _returnvalue (`KismetMathLibrary.MakeRotator` 0.0 0.0 180.0)))))))
        (:`<`
          (goto _label_5))))
    (:`then_2`
      (`self.ProcessGlowRecharge`))))

(event `InputAxis|MoveRight`
  (params (AxisValue :type "Float (single-precision)"))
  ;[1 1 1] Handle movement
  (if (not (`self.Dead`))
    (if (> AxisValue 0.0)
      (set `self.isMovingRight` true)
      (elif (< AxisValue 0.0)
        (set `self.isMovingRight` false)))
    (`self.AddMovementInput` (1.0 0.0 0.0) AxisValue)))

(event `self.GlowLongPulse.OnComponentBeginOverlap`
  (params (OverlappedComponent :type "PrimitiveComponent Object Reference") (OtherActor :type "Actor Object Reference") (OtherComp :type "PrimitiveComponent Object Reference") (OtherBodyIndex :type Integer) (bFromSweep :type Boolean) (SweepResult :type "HitResult Structure (by ref)")))

(event `self.GlowLong.OnComponentBeginOverlap`
  (params (OverlappedComponent :type "PrimitiveComponent Object Reference") (OtherActor :type "Actor Object Reference") (OtherComp :type "PrimitiveComponent Object Reference") (OtherBodyIndex :type Integer) (bFromSweep :type Boolean) (SweepResult :type "HitResult Structure (by ref)")))

(fn `CalculateWallDamage`
  (returns (Damage :type Integer))
  (return (`KismetMathLibrary.Round` (* 2 (`KismetMathLibrary.GetMaxElement` (`SceneComponent.K2_GetComponentScale` (`self.GlowLongPulse`)))))))

(fn `CanUseGlow`
  (params (ShortPulse :type Boolean) (LongPulse :type Boolean) (LongGlow :type Boolean))
  (returns (CanUseShortPulse :type Boolean) (CanUseLongPulse :type Boolean) (CanUseLongGlow :type Boolean))
  (locals (ShortPulseLocal :type Boolean) (LongPulseLocal :type Boolean) (LongGlowLocal :type Boolean))
  (if (and (`self.GlowShortPulseCharged`) (and (> (`self.ShortPulseHealth`) 0) (not (or (`self.GlowLongActive`) (`self.GlowLongPulseActive`)))) ShortPulse)
    (return true false false)
    (elif (and (`self.GlowLongPulseCharged`) (and (> (`self.LongPulseHealth`) 0) (not (or (`self.GlowShortPulseActive`) (`self.GlowLongActive`)))) LongPulse)
      (return false true false)
      (elif (and (`self.GlowLongCharged`) (and (> (`self.LongHealth`) 0) (not (or (`self.GlowShortPulseActive`) (`self.GlowLongPulseActive`)))) LongGlow)
        (return false false true)
        (else
          (return false false false))))))

(fn `ChangeFlipBook`
  (params (`ToChange To` :type "PaperFlipbook Object Reference"))
  ;[1 1 1] If Yugen is moving
  (if (> (`KismetMathLibrary.VSize` (`CharacterMovementComponent.GetCurrentAcceleration` (`self.CharacterMovement`))) 0.0)
    ;[1 1 1] Is Yugen in the air?
    (if (or (`NavMovementComponent.IsFalling` (`self.CharacterMovement`)) (`NavMovementComponent.IsFlying` (`self.CharacterMovement`)))
      ;[1 1 1] Is Yugen going down?
      (if (< (.z (`self.GetVelocity`)) 0.0)
        ;[1 1 1] Falling Side
        (bind _flipbookalreadyenabled (`self.CompareFlipbook` "/Game/Yugen/Assets/Sprites/Yugen/FallSide/Frames/yugenFallSide.yugenFallSide"))
        (if (not _flipbookalreadyenabled)
          (`PaperFlipbookComponent.SetFlipbook` (`self.Sprite`) "/Game/Yugen/Assets/Sprites/Yugen/FallSide/Frames/yugenFallSide.yugenFallSide"))
        (else
          ;[1 1 1] Jump Side
          (bind _flipbookalreadyenabled_2 (`self.CompareFlipbook` "/Game/Yugen/Assets/Sprites/Yugen/JumpSide/Frames/yugenJumpSide.yugenJumpSide"))
          (if (not _flipbookalreadyenabled_2)
            (`PaperFlipbookComponent.SetFlipbook` (`self.Sprite`) "/Game/Yugen/Assets/Sprites/Yugen/JumpSide/Frames/yugenJumpSide.yugenJumpSide"))))
      (else
        ;[1 1 1] Is Yugen Long glow?
        (if (`self.GlowLongActive`)
          ;[1 1 1] Long Glow
          (bind _flipbookalreadyenabled_3 (`self.CompareFlipbook` "/Game/Yugen/Assets/Sprites/Yugen/LongGlow/Frames/yugenLongGlow.yugenLongGlow"))
          (if (not _flipbookalreadyenabled_3)
            (`PaperFlipbookComponent.SetFlipbook` (`self.Sprite`) "/Game/Yugen/Assets/Sprites/Yugen/LongGlow/Frames/yugenLongGlow.yugenLongGlow"))
          (else
            ;[1 1 1] Walking
            (bind _flipbookalreadyenabled_4 (`self.CompareFlipbook` "/Game/Yugen/Assets/Sprites/Yugen/WalkV2/Frames/yugenWalk.yugenWalk"))
            (if (not _flipbookalreadyenabled_4)
              (`PaperFlipbookComponent.SetFlipbook` (`self.Sprite`) "/Game/Yugen/Assets/Sprites/Yugen/WalkV2/Frames/yugenWalk.yugenWalk"))))))
    (else
      ;[1 1 1] Is Yugen in the air?
      (if (or (`NavMovementComponent.IsFalling` (`self.CharacterMovement`)) (`NavMovementComponent.IsFlying` (`self.CharacterMovement`)))
        ;[1 1 1] Is Yugen going down?
        (if (< (.z (`self.GetVelocity`)) 0.0)
          ;[1 1 1] FallingFront
          (bind _flipbookalreadyenabled_5 (`self.CompareFlipbook` "/Game/Yugen/Assets/Sprites/Yugen/FallFront/Frames/yugenFallFront.yugenFallFront"))
          (if (not _flipbookalreadyenabled_5)
            (`PaperFlipbookComponent.SetFlipbook` (`self.Sprite`) "/Game/Yugen/Assets/Sprites/Yugen/FallFront/Frames/yugenFallFront.yugenFallFront"))
          (else
            ;[1 1 1] Jump Front
            (bind _flipbookalreadyenabled_6 (`self.CompareFlipbook` "/Game/Yugen/Assets/Sprites/Yugen/JumpFront/Frames/yugenJumpFront.yugenJumpFront"))
            (if (not _flipbookalreadyenabled_6)
              (`PaperFlipbookComponent.SetFlipbook` (`self.Sprite`) "/Game/Yugen/Assets/Sprites/Yugen/JumpFront/Frames/yugenJumpFront.yugenJumpFront"))))
        (else
          ;[1 1 1] Is Yugen glowing?
          (if (or (`self.GlowShortPulseActive`) (`self.GlowLongPulseActive`))
            ;[1 1 1] Glowing
            (bind _flipbookalreadyenabled_7 (`self.CompareFlipbook` "/Game/Yugen/Assets/Sprites/Yugen/GlowPulseAndShortGlow/Frames/yugenGlow.yugenGlow"))
            (if (not _flipbookalreadyenabled_7)
              (`PaperFlipbookComponent.SetFlipbook` (`self.Sprite`) "/Game/Yugen/Assets/Sprites/Yugen/GlowPulseAndShortGlow/Frames/yugenGlow.yugenGlow"))
            (else
              ;[1 1 1] Not moving
              (bind _flipbookalreadyenabled_8 (`self.CompareFlipbook` "/Game/Yugen/Assets/Sprites/Yugen/Idle/Frames/yugenIdle.yugenIdle"))
              (if (not _flipbookalreadyenabled_8)
                (`PaperFlipbookComponent.SetFlipbook` (`self.Sprite`) "/Game/Yugen/Assets/Sprites/Yugen/Idle/Frames/yugenIdle.yugenIdle")))))))))

(fn `CompareFlipbook`
  (params (Flipbook :type "PaperFlipbook Object Reference"))
  (returns (FlipbookAlreadyEnabled :type Boolean))
  (return (== Flipbook (`PaperFlipbookComponent.GetFlipbook` (`self.Sprite`)))))

(fn `ExpandGlow`
  (params (Glow :type "SphereComponent Object Reference") (ShortPulse :type Boolean) (LongPulse :type Boolean) (LongGlow :type Boolean))
  (locals (ShortPulseLocal :type Boolean) (LongPulseLocal :type Boolean) (LongGlowLocal :type Boolean) (GlowLocal :type "SphereComponent Object Reference"))
  (bind _scale (`self.Scale`))
  (bind (_returnvalue_x _returnvalue_y _returnvalue_z) (`KismetMathLibrary.BreakVector` (`SceneComponent.K2_GetComponentScale` (`local.GlowLocal`))))
  ;[1 1 1] Make glow bigger if active, set small if inactive
  (set `local.GlowLocal` Glow)
  (if ShortPulse
    (set `self.Scale` 0.2)
    (set `self.MaxRadius` 300.0)
    (else
      (set `self.Scale` 0.1)
      (set `self.MaxRadius` 600.0)))
  (if (or ShortPulse LongPulse LongGlow)
    (if (< (`SphereComponent.GetScaledSphereRadius` (`local.GlowLocal`)) (`self.MaxRadius`))
      (`SceneComponent.SetWorldScale3D` (`local.GlowLocal`) (`KismetMathLibrary.MakeVector` (+ _returnvalue_x _scale) (+ _returnvalue_y _scale) (+ _returnvalue_z _scale))))))

(fn `ProcessGlowDamage`
  (params (GlowHealth :type "Integer (by ref)"))
  (returns (EndHealth :type Integer))
  ;[1 1 1] decrement a glows damage if it's not 0
  (if (<= GlowHealth 0)
    (return 0)
    (else
      (return (- GlowHealth 1)))))

(fn `ProcessGlowRecharge`
  ;[1 1 1] Calculate Long Pulse Glow
  (if (or (or (`self.GlowLongPulseActive`) (`self.GlowLongPulseCharged`)) (== (`self.LongPulseHealth`) 0))
    ;[1 1 1] Calculate Short Pulse Glow
    (if (or (or (`self.GlowShortPulseCharged`) (`self.GlowShortPulseActive`)) (== (`self.ShortPulseHealth`) 0))
      ;[1 1 1] Calculate Long Glow
      (if (or (or (`self.GlowLongActive`) (`self.GlowLongCharged`)) (== (`self.LongHealth`) 0))
        _
        (elif (< (`self.GlowLongCountdownToRecharge`) 300)
          (bind _result (`/Engine/EditorBlueprintResources/StandardMacros.IncrementInt` (`self.GlowLongCountdownToRecharge`))
            (:`  `
              (bind _output_get (set `self.GlowLongRechargeAmount` _result))
              (`KismetSystemLibrary.PrintText` "Long Glow: ")
              (`KismetSystemLibrary.PrintString` (`KismetStringLibrary.Conv_IntToString` _output_get))))
          (else
            (bind _result_2 (`/Engine/EditorBlueprintResources/StandardMacros.IncrementInt` (`self.GlowLongRechargeAmount`))
              (:`  `
                (set `self.GlowLongRechargeAmount` _result_2)
                (if (>= (`self.GlowLongRechargeAmount`) 300)
                  (set `self.GlowLongCharged` true)
                  (set `self.GlowLongCountdownToRecharge` 0)
                  (set `self.GlowLongRechargeAmount` 0)))))))
      (elif (< (`self.GlowShortPulseCountdownToRecharge`) 60)
        (bind _result_3 (`/Engine/EditorBlueprintResources/StandardMacros.IncrementInt` (`self.GlowShortPulseCountdownToRecharge`))
          (:`  `
            (bind _output_get_2 (set `self.GlowShortPulseCountdownToRecharge` _result_3))
            (`KismetSystemLibrary.PrintText` "Short Pulse: ")
            (`KismetSystemLibrary.PrintString` (`KismetStringLibrary.Conv_IntToString` _output_get_2))))
        (else
          (bind _result_4 (`/Engine/EditorBlueprintResources/StandardMacros.IncrementInt` (`self.GlowShortPulseRechargeAmount`))
            (:`  `
              (set `self.GlowShortPulseRechargeAmount` _result_4)
              (if (>= (`self.GlowShortPulseRechargeAmount`) 60)
                (set `self.GlowShortPulseCharged` true)
                (set `self.GlowShortPulseCountdownToRecharge` 0)
                (set `self.GlowShortPulseRechargeAmount` 0)))))))
    (elif (< (`self.GlowLongPulseCountdownToRecharge`) 120)
      (bind _result_5 (`/Engine/EditorBlueprintResources/StandardMacros.IncrementInt` (`self.GlowLongPulseCountdownToRecharge`))
        (:`  `
          (bind _output_get_3 (set `self.GlowLongPulseCountdownToRecharge` _result_5))
          (`KismetSystemLibrary.PrintText` "Long Pulse: ")
          (`KismetSystemLibrary.PrintString` (`KismetStringLibrary.Conv_IntToString` _output_get_3))))
      (else
        (bind _result_6 (`/Engine/EditorBlueprintResources/StandardMacros.IncrementInt` (`self.GlowLongPulseRechargeAmount`))
          (:`  `
            (set `self.GlowLongPulseRechargeAmount` _result_6)
            (if (>= (`self.GlowLongPulseRechargeAmount`) 60)
              (set `self.GlowLongPulseCharged` true)
              (set `self.GlowLongPulseCountdownToRecharge` 0)
              (set `self.GlowLongPulseRechargeAmount` 0))))))))

(fn `ResetGlow`
  (params (Glow :type "SphereComponent Object Reference"))
  (`SceneComponent.SetWorldScale3D` Glow (0.25 0.25 0.25)))

(fn `TakeDamage`
  (set `self.ShortPulseHealth` (- (`self.ShortPulseHealth`) 1))
  (`KismetSystemLibrary.PrintString` "ouch!")
  (set `self.Dead` (and (== (`self.LongHealth`) 0) (and (== (`self.ShortPulseHealth`) 0) (== (`self.LongPulseHealth`) 0)))))

(fn `UpdateAnimation`)

(fn `UserConstructionScript`)