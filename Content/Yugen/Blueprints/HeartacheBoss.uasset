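; Heartache boss enemy that chases the player with AI MoveTo, animated through flipbook swaps.
; Box overlap with the player's body triggers an attack that knocks the player back, deals damage and starts a timed cooldown, which halts further move orders.
; During cooldown, overlapping the player's sphere component while the short glow pulse is active costs one health, or plays death and destroys the boss on the last point.
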(event `self.Box.OnComponentBeginOverlap`
  (params (OverlappedComponent :type "PrimitiveComponent Object Reference") (OtherActor :type "Actor Object Reference") (OtherComp :type "PrimitiveComponent Object Reference") (OtherBodyIndex :type Integer) (bFromSweep :type Boolean) (SweepResult :type "HitResult Structure (by ref)"))
  (bind _sprite (`self.Sprite`))
  (bind _returnvalue (`PaperFlipbookComponent.GetFlipbookLength` _sprite))
  ;[1 1 1] Collide with character
  (if (not (and (`self.Colliding`) (`self.NotCooldown`)))
    (bind _asplayer_character (cast `/Game/Yugen/Blueprints/PlayerCharacter` OtherActor))
    (set `self.Colliding` true)
    (cast `SphereComponent` OtherComp
      (:`then`
        ;[1 1 1] Take damage and die
        (if (and (not (`self.NotCooldown`)) (`/Game/Yugen/Blueprints/PlayerCharacter.GlowShortPulseActive` _asplayer_character))
          (if (> (`self.Heartache Health`) 1)
            (`PaperFlipbookComponent.SetFlipbook` _sprite "/Game/Yugen/Assets/Flipbooks/Boss/Heartache/Damage/HeartacheDamage1.HeartacheDamage1")
            (`KismetSystemLibrary.Delay` _returnvalue)
            (`self.Heartache Take Damage` self)
            (`PaperFlipbookComponent.SetFlipbook` _sprite "/Game/Yugen/Assets/Flipbooks/Boss/Heartache/Idle/HeartacheIdle1.HeartacheIdle1")
            (set `self.Colliding` false)
            (else
              (`self.SetActorEnableCollision` self false)
              (`PaperFlipbookComponent.SetFlipbook` _sprite "/Game/Yugen/Assets/Flipbooks/Boss/Heartache/Death/HeartacheDeath1.HeartacheDeath1")
              (`KismetSystemLibrary.Delay` _returnvalue)
              (`self.K2_DestroyActor` self)))
          (else
            (set `self.Colliding` false))))
      (:`CastFailed`
        (if (`self.NotCooldown`)
          (`PaperFlipbookComponent.SetFlipbook` (`self.Sprite`) "/Game/Yugen/Assets/Flipbooks/Boss/Heartache/Attack/HeartacheAttack1.HeartacheAttack1")
          (`self.LaunchCharacter` _asplayer_character (`KismetMathLibrary.MakeVector` (* (.x (`.Normal` (`GameplayStatics.BreakHitResult` SweepResult))) -1500.0) 0.0 400.0) false false)
          (`/Game/Yugen/Blueprints/PlayerCharacter.TakeDamage` _asplayer_character)
          (`KismetSystemLibrary.Delay` (`PaperFlipbookComponent.GetFlipbookLength` (`self.Sprite`)))
          (set `self.NotCooldown` false)
          (`PaperFlipbookComponent.SetFlipbook` (`self.Sprite`) "/Game/Yugen/Assets/Flipbooks/Boss/Heartache/Cooldown/HeartacheCooldown1.HeartacheCooldown1")
          (`KismetSystemLibrary.PrintString` (`KismetSystemLibrary.GetDisplayName` (`PaperFlipbookComponent.GetFlipbook` (`self.Sprite`))))
          (`KismetSystemLibrary.Delay` 5.0)
          (set `self.NotCooldown` true)
          (set `self.Colliding` false)
          (else
            (set `self.Colliding` false)))))))

(event `self.ReceiveTick`
  (params (DeltaSeconds :type "Float (single-precision)"))
  (bind _sprite (`self.Sprite`))
  ;[1 1 1] Flip character
  (if (not (`self.Flipped`))
    (`SceneComponent.K2_SetWorldRotation` _sprite (struct :`Yaw` 180.0) false false)
    (set `self.Flipped` true))
  ;[1 1 1] Chase character
  (if (and (not (`self.Colliding`)) (`self.NotCooldown`))
    (`PaperFlipbookComponent.SetFlipbook` _sprite "/Game/Yugen/Assets/Flipbooks/Boss/Heartache/Run/HeartacheRun1.HeartacheRun1")
    (`|AIMoveTo` self (0.0 0.0 0.0) (`GameplayStatics.GetPlayerCharacter` 0) 100.0 true)))

(fn `Compare Flipbook`
  (params (Flipbook :type "PaperFlipbook Object Reference"))
  (returns (FlipbookAlreadyEnabled :type Boolean))
  (return (== Flipbook (`PaperFlipbookComponent.GetFlipbook` (`self.Sprite`)))))

(fn `Heartache Take Damage`
  ;[0.474 0 0.03306] Take damage
  (set `self.Heartache Health` (- (`self.Heartache Health`) 1)))

(fn `UserConstructionScript`)