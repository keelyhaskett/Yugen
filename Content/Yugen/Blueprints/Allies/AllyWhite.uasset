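; AllyWhite is an ally that patrols between two points and recharges the player's health on contact.
; The construction script builds InterpToMovement's path from PointA and PointB, and a FlipFlop turns the sprite on each reversal.
; Overlapping the player stops movement, sets ShortPulseHealth to a fixed value, and plays the regen flipbook before switching to idle.
; Sphere components and non-player Paper characters only trigger a debug print.
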(event `self.InterpToMovement.OnInterpToReverse`
  (params (ImpactResult :type "HitResult Structure (by ref)") (Time :type "Float (single-precision)"))
  (bind _sprite (`self.Sprite`))
  ;[1 1 1] Turn when walking
  (`/Engine/EditorBlueprintResources/StandardMacros.FlipFlop`
    (:`A`
      (`SceneComponent.K2_SetWorldRotation` _sprite (struct :`Yaw` 180.0) false false))
    (:`B`
      (`SceneComponent.K2_SetWorldRotation` :`self` _sprite))))

(event `self.Collision.OnComponentBeginOverlap`
  (params (OverlappedComponent :type "PrimitiveComponent Object Reference") (OtherActor :type "Actor Object Reference") (OtherComp :type "PrimitiveComponent Object Reference") (OtherBodyIndex :type Integer) (bFromSweep :type Boolean) (SweepResult :type "HitResult Structure (by ref)"))
  ;[1 1 1] Stop when meeting player
  (cast `SphereComponent` OtherComp
    (:`then`
      (`KismetSystemLibrary.PrintString` "thats not u!" :!label _label))
    (:`CastFailed`
      (bind _aspaper_character (cast `PaperCharacter` OtherActor))
      (bind _asplayer_character (cast `/Game/Yugen/Blueprints/PlayerCharacter` _aspaper_character)
        (:`then`
          (`InterpToMovementComponent.StopSimulating` (`self.InterpToMovement`) SweepResult)
          (`MovementComponent.StopMovementImmediately` (`self.CharacterMovement`))
          (`self.Give health` _asplayer_character)
          (`KismetSystemLibrary.Delay` (`PaperFlipbookComponent.GetFlipbookLength` (`self.Sprite`)))
          (`PaperFlipbookComponent.SetFlipbook` (`self.Sprite`) "/Game/Yugen/Assets/Flipbooks/Ally/White/Idle/Frames/allyIdleWhite.allyIdleWhite"))
        (:`CastFailed`
          (goto _label))))))

(fn `Give health`
  (params (Target :type "/Game/Yugen/Blueprints/PlayerCharacter Object Reference"))
  ;[1 1 1] Recharges long pulse health
  (set `/Game/Yugen/Blueprints/PlayerCharacter.ShortPulseHealth` 10 Target)
  (`KismetSystemLibrary.PrintString` "mwah!")
  (`PaperFlipbookComponent.SetFlipbook` (`self.Sprite`) "/Game/Yugen/Assets/Flipbooks/Ally/White/Regen/Frames/allyRegenWhite.allyRegenWhite"))

(fn `UserConstructionScript`
  (set `InterpToMovementComponent.ControlPoints` (`|MakeArray` (make `InterpControlPoint` (`self.Point A`)) (make `InterpControlPoint` (`self.Point B`))) (`self.InterpToMovement`)))