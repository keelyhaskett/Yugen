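; Fake glow actor that builds a procedural, radial light mesh shaped by the surrounding geometry.
; Each tick it sweeps visibility line traces in a vertical circle by rotating pitch, placing fan vertices at hits or at full light distance.
; UVs store normalized distance for the glow material; the mesh section is created once, then updated.
; A delayed check pushes LightColor changes to the dynamic material instance.
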(event `self.ReceiveBeginPlay`
  (set `self.LineTraceAngle` (/ 360.0 (`KismetMathLibrary.Conv_IntToDouble` (`self.Polygon`))))
  (set `self.OriginalColor` (`self.LightColor`)))

(event `self.ReceiveTick`
  (params (DeltaSeconds :type "Float (single-precision)"))
  (bind _returnvalue (`self.K2_GetActorLocation`))
  (bind _returnvalue_2 (`self.K2_GetActorLocation`))
  (`|ExecutionSequence`
    (:`then_0`
      (`KismetArrayLibrary.Array_Clear` (`self.UVs`))
      (`KismetArrayLibrary.Array_Clear` (`self.Triangles`))
      (`KismetArrayLibrary.Array_Clear` (`self.Vertices`))
      (`KismetArrayLibrary.Array_Add` (`self.Vertices`))
      (`KismetArrayLibrary.Array_Add` (`self.UVs`))
      (set `self.EndVector` (`KismetMathLibrary.MakeVector` (`self.LightDistance`)))
      (for _ (range (+ (`self.Polygon`) 1))
        (bind (_outhit _returnvalue_3) (`KismetSystemLibrary.LineTraceSingle` _returnvalue_2 (+ _returnvalue_2 (`self.EndVector`)) "TraceTypeQuery1"))
        (set `self.LineTraceReturn` _returnvalue_3)
        (bind (_bblockinghit _binitialoverlap _time _distance _location _impactpoint _normal _impactnormal _physmat _hitactor _hitcomponent _hitbonename _hititem _faceindex _tracestart _traceend) (`GameplayStatics.BreakHitResult` _outhit))
        (set `self.LineTraceLocation` (- _location _returnvalue))
        (set `self.LineTraceEnd` (- _traceend _returnvalue))
        (set `self.EndVector` (`KismetMathLibrary.GreaterGreater_VectorRotator` (`self.EndVector`) (`KismetMathLibrary.MakeRotator` 0.0 (`self.LineTraceAngle`))))
        (if (`self.LineTraceReturn`)
          (`KismetArrayLibrary.Array_Add` (`self.Vertices`) (`self.LineTraceLocation`))
          (`KismetArrayLibrary.Array_Add` (`self.UVs`) (`KismetMathLibrary.MakeVector2D` (`KismetMathLibrary.MapRangeClamped` (`KismetMathLibrary.VSize` (`self.LineTraceLocation`)) 0.0 (`self.LightDistance`) 0.0 1.0)))
          (else
            (`KismetArrayLibrary.Array_Add` (`self.Vertices`) (`self.LineTraceEnd`))
            (`KismetArrayLibrary.Array_Add` (`self.UVs`) (1.0 0.0)))))
      (set `self.TriangleOffset` 1)
      (for _ (range (+ (- (`KismetArrayLibrary.Array_Length` (`self.Vertices`)) 3) 1))
        (`KismetArrayLibrary.Array_Add` (`self.Triangles`))
        (for _index (range 2)
          (`KismetArrayLibrary.Array_Add` (`self.Triangles`) (+ _index (`self.TriangleOffset`))))
        (`/Engine/EditorBlueprintResources/StandardMacros.IncrementInt` (`self.TriangleOffset`)))
      (if (`self.CreatedMesh`)
        (`ProceduralMeshComponent.UpdateMeshSection_LinearColor` :`self` (`self.ProceduralMesh`) :`Vertices` (`self.Vertices`) :`UV0` (`self.UVs`))
        (else
          (`ProceduralMeshComponent.CreateMeshSection_LinearColor` :`self` (`self.ProceduralMesh`) :`Vertices` (`self.Vertices`) :`Triangles` (`self.Triangles`) :`UV0` (`self.UVs`))
          (`PrimitiveComponent.SetMaterial` (`self.ProceduralMesh`) 0 "/Game/Yugen/Blueprints/GlowComponents/FakeGlow_Mat.FakeGlow_Mat")
          (bind _returnvalue_4 (`PrimitiveComponent.CreateDynamicMaterialInstance` (`self.ProceduralMesh`) 0 null "None"))
          (`MaterialInstanceDynamic.SetVectorParameterValue` _returnvalue_4 "LightColor" (`self.LightColor`) :!label _label)
          (set `self.CreatedMesh` true))))
    (:`then_1`
      (`KismetSystemLibrary.Delay` 0.2)
      (if (not (== (`self.LightColor`) (`self.OriginalColor`)))
        (`self.UpdateColor`)
        (set `self.OriginalColor` (`self.LightColor`))))))

(event `UpdateColor`
  (goto _label))

(fn `UserConstructionScript`)