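; Short pulse glow actor that follows the player, charging a glow radius and releasing it as a burst of light.
; Each Tick, while GlowShortPulseActive is set, Grow scales the collision and range spheres, clearing the flag at max radius.
; Otherwise, Pop hides the range sphere and widens the light toward ReleaseRadius, then Fade dims it and destroys the actor.
; Grow's early-release radius capture is unreachable from Tick's active-only call.
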(event `self.ReceiveTick`
  (params (DeltaSeconds :type "Float (single-precision)"))
  (bind _asplayer_character (cast `/Game/Yugen/Blueprints/PlayerCharacter` (`GameplayStatics.GetPlayerPawn` 0)))
  (`|ExecutionSequence`
    (:`then_0`
      (if (`/Game/Yugen/Blueprints/PlayerCharacter.GlowShortPulseActive` _asplayer_character)
        (`self.Grow` _asplayer_character)
        (else
          (`self.Pop` _asplayer_character (`self.ReleaseRadius`))
          (if (`self.Popped`)
            (`self.Fade`)))))
    (:`then_1`
      (bind (_returnvalue_x _returnvalue_y _returnvalue_z) (`KismetMathLibrary.BreakVector` (`SceneComponent.K2_GetComponentLocation` (`Character.CapsuleComponent` _asplayer_character))))
      (`self.K2_SetActorLocation` (`KismetMathLibrary.MakeVector` _returnvalue_x (+ _returnvalue_y -1.0) _returnvalue_z)))))

(fn `Fade`
  (bind _returnvalue (- (`LightComponentBase.Intensity` (`self.Glow`)) 0.4))
  (`SceneComponent.SetVisibility` (`self.RangeSphere`) false false)
  (`LightComponent.SetIntensity` (`self.Glow`) _returnvalue)
  (if (<= _returnvalue 0.0)
    (`self.K2_DestroyActor`)))

(fn `Grow`
  (params (Player :type "/Game/Yugen/Blueprints/PlayerCharacter Object Reference"))
  (locals (PlayerLocal :type "/Game/Yugen/Blueprints/PlayerCharacter Object Reference"))
  (bind _glowcollision (`self.GlowCollision`))
  (bind _rangesphere (`self.RangeSphere`))
  (bind (_returnvalue_x _returnvalue_y _returnvalue_z) (`KismetMathLibrary.BreakVector` (`SceneComponent.K2_GetComponentScale` _rangesphere)))
  (bind (_returnvalue_x_2 _returnvalue_y_2 _returnvalue_z_2) (`KismetMathLibrary.BreakVector` (`SceneComponent.K2_GetComponentScale` _glowcollision)))
  (set `local.PlayerLocal` Player)
  (if (`/Game/Yugen/Blueprints/PlayerCharacter.GlowShortPulseActive` Player)
    (if (< (`SphereComponent.GetScaledSphereRadius` (`self.GlowCollision`)) (`self.MaxRadius`))
      (`SceneComponent.SetWorldScale3D` _glowcollision (`KismetMathLibrary.MakeVector` (+ _returnvalue_x_2 0.2) (+ _returnvalue_y_2 0.2) (+ _returnvalue_z_2 0.2)))
      (`SceneComponent.SetWorldScale3D` _rangesphere (`KismetMathLibrary.MakeVector` (+ _returnvalue_x 0.2) (+ _returnvalue_y 0.2) (+ _returnvalue_z 0.2)))
      (else
        (set `self.ReleaseRadius` (`self.MaxRadius`))
        (set `/Game/Yugen/Blueprints/PlayerCharacter.GlowShortPulseActive` false (`local.PlayerLocal`) :!label _label)))
    (else
      (set `self.ReleaseRadius` (`SphereComponent.GetScaledSphereRadius` (`self.GlowCollision`)))
      (goto _label))))

(fn `Pop`
  (params (Player :type "/Game/Yugen/Blueprints/PlayerCharacter Object Reference") (Radius :type "Float (double-precision)"))
  (bind _glow (`self.Glow`))
  (bind _returnvalue (* (`LocalLightComponent.AttenuationRadius` _glow) 1.3))
  (`SceneComponent.SetVisibility` (`self.RangeSphere`) false false)
  (if (> Radius _returnvalue)
    (set `self.Popped` false)
    (`LocalLightComponent.SetAttenuationRadius` _glow (+ _returnvalue 100.0))
    (else
      (set `self.Popped` true))))

(fn `UserConstructionScript`)