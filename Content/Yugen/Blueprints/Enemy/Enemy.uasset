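; Paper2D enemy that patrols between two points, chases the player and trades damage on contact.
; InterpToMovement drives the patrol from construction-script points, while Sensing overlaps start AIMoveTo chases or return it to idle.
; Capsule overlaps knock back and hurt the player, unless the player's glow sphere is hit, whose active short pulse damages or kills the enemy.
; State booleans, current-flipbook checks and flipbook-length delays gate and time reactions.
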(event `self.InterpToMovement.OnInterpToReverse`
  (params (ImpactResult :type "HitResult Structure (by ref)") (Time :type "Float (single-precision)"))
  (bind _sprite (`self.Sprite`))
  ;[1 1 1] Turn around
  (`/Engine/EditorBlueprintResources/StandardMacros.FlipFlop`
    (:`A`
      (`SceneComponent.K2_SetWorldRotation` _sprite (struct :`Yaw` 180.0) false false))
    (:`B`
      (`SceneComponent.K2_SetWorldRotation` :`self` _sprite)))
  (`PaperFlipbookComponent.SetFlipbook` _sprite "/Game/Yugen/Assets/Flipbooks/Enemy/EnemyWalk/Frames/enemyWalk.enemyWalk"))

(event `self.Capsule.OnComponentBeginOverlap`
  (params (OverlappedComponent :type "PrimitiveComponent Object Reference") (OtherActor :type "Actor Object Reference") (OtherComp :type "PrimitiveComponent Object Reference") (OtherBodyIndex :type Integer) (bFromSweep :type Boolean) (SweepResult :type "HitResult Structure (by ref)"))
  (bind _sprite (`self.Sprite`))
  (bind _sprite_2 (`self.Sprite`))
  (bind _sprite_3 (`self.Sprite`))
  ;[1 1 1] Collide with character
  ;[1 1 1] Collide with glow and take damage or die
  (cast `SphereComponent` OtherComp
    (:`then`
      (bind _asplayer_character (cast `/Game/Yugen/Blueprints/PlayerCharacter` OtherActor))
      (if (`/Game/Yugen/Blueprints/PlayerCharacter.GlowShortPulseActive` _asplayer_character)
        (if (> (`self.Enemy Health`) 1)
          (bind _flipbookalreadyenabled (`self.Compare Flipbook` self "/Game/Yugen/Assets/Flipbooks/Enemy/EnemyDamage/Frames/enemyDamage.enemyDamage"))
          (set `self.NotBeingDamaged` false)
          (if (not _flipbookalreadyenabled)
            (`InterpToMovementComponent.StopSimulating` (`self.InterpToMovement`) SweepResult)
            (`NavMovementComponent.StopActiveMovement` (`self.CharacterMovement`))
            (`self.Enemy Take Damage` self)
            (`PaperFlipbookComponent.SetFlipbook` _sprite "/Game/Yugen/Assets/Flipbooks/Enemy/EnemyDamage/Frames/enemyDamage.enemyDamage")
            (`KismetSystemLibrary.Delay` (`PaperFlipbookComponent.GetFlipbookLength` _sprite))
            (set `self.NotBeingDamaged` true)
            (`PaperFlipbookComponent.SetFlipbook` (`self.Sprite`) "/Game/Yugen/Assets/Flipbooks/Enemy/EnemyIdle/Frames/enemyIdle.enemyIdle")
            (set `self.isIdle` true)
            (`CharacterMovementComponent.SetMovementMode` (`self.CharacterMovement`) "MOVE_NavWalking" 0))
          (else
            (set `self.NotDying` false)
            (`ActorComponent.SetComponentTickEnabled` (`self.InterpToMovement`) false)
            (`self.SetActorEnableCollision` self false)
            (`CharacterMovementComponent.DisableMovement` (`self.CharacterMovement`))
            (`PaperFlipbookComponent.SetFlipbook` _sprite_2 "/Game/Yugen/Assets/Flipbooks/Enemy/EnemyDamage/Frames/enemyDamage.enemyDamage")
            (`KismetSystemLibrary.Delay` (`PaperFlipbookComponent.GetFlipbookLength` _sprite_2))
            (`self.K2_DestroyActor` self)))))
    (:`CastFailed`
      (if (and (`self.NotDying`) (`self.NotBeingDamaged`))
        (bind _asplayer_character_2 (cast `/Game/Yugen/Blueprints/PlayerCharacter` OtherActor))
        (`self.LaunchCharacter` _asplayer_character_2 (`KismetMathLibrary.MakeVector` (* (.x (`.Normal` (`GameplayStatics.BreakHitResult` SweepResult))) -1500.0)) false false)
        (`PaperFlipbookComponent.SetFlipbook` (`self.Sprite`) "/Game/Yugen/Assets/Flipbooks/Enemy/EnemyAttack/Frames/enemyAttack.enemyAttack")
        (`/Game/Yugen/Blueprints/PlayerCharacter.TakeDamage` _asplayer_character_2)
        (`KismetSystemLibrary.Delay` (`PaperFlipbookComponent.GetFlipbookLength` _sprite_3))
        (`PaperFlipbookComponent.SetFlipbook` _sprite_3 "/Game/Yugen/Assets/Flipbooks/Enemy/EnemyIdle/Frames/enemyIdle.enemyIdle")
        (set `self.isIdle` true)))))

(event `self.Sensing.OnComponentBeginOverlap`
  (params (OverlappedComponent :type "PrimitiveComponent Object Reference") (OtherActor :type "Actor Object Reference") (OtherComp :type "PrimitiveComponent Object Reference") (OtherBodyIndex :type Integer) (bFromSweep :type Boolean) (SweepResult :type "HitResult Structure (by ref)"))
  (bind _returnvalue_x (`KismetMathLibrary.BreakVector` (`SceneComponent.K2_GetComponentLocation` (`self.CapsuleComponent`))))
  (bind _returnvalue (and (`self.NotDying`) (`self.NotBeingDamaged`)))
  ;[1 1 1] Chase Character
  (cast `SphereComponent` OtherComp
    (:`CastFailed`
      (bind _output_get (set `self.Other Actor` OtherActor))
      (bind _asplayer_character (cast `/Game/Yugen/Blueprints/PlayerCharacter` _output_get))
      (bind _returnvalue_x_2 (`KismetMathLibrary.BreakVector` (`SceneComponent.K2_GetComponentLocation` (`Character.CapsuleComponent` _asplayer_character))))
      (if (>= (- _returnvalue_x _returnvalue_x_2) 0.0)
        (if _returnvalue
          (set `self.isIdle` false)
          (`PaperFlipbookComponent.SetFlipbook` (`self.Sprite`) "/Game/Yugen/Assets/Flipbooks/Enemy/EnemyWalk/Frames/enemyChase.enemyChase" :!label _label)
          (`InterpToMovementComponent.StopSimulating` (`self.InterpToMovement`) SweepResult)
          (`|AIMoveTo` self (0.0 0.0 0.0) (`self.Other Actor`) 0.0 true
            (:`OnSuccess`
              _)
            (:`OnFail`
              _))
          (`PaperFlipbookComponent.SetFlipbook` (`self.Sprite`) "/Game/Yugen/Assets/Flipbooks/Enemy/EnemyIdle/Frames/enemyIdle.enemyIdle")
          (set `self.isIdle` true))
        (elif _returnvalue
          (set `self.isIdle` false)
          (goto _label))))))

(event `self.Sensing.OnComponentEndOverlap`
  (params (OverlappedComponent :type "PrimitiveComponent Object Reference") (OtherActor :type "Actor Object Reference") (OtherComp :type "PrimitiveComponent Object Reference") (OtherBodyIndex :type Integer))
  ;[1 1 1] Stop chasing
  (cast `/Game/Yugen/Blueprints/PlayerCharacter` OtherActor)
  (cast `SphereComponent` OtherComp
    (:`CastFailed`
      (bind _flipbookalreadyenabled (`self.Compare Flipbook` self "/Game/Yugen/Assets/Flipbooks/Enemy/EnemyWalk/Frames/enemyChase.enemyChase"))
      (if _flipbookalreadyenabled
        (`PaperFlipbookComponent.SetFlipbook` (`self.Sprite`) "/Game/Yugen/Assets/Flipbooks/Enemy/EnemyIdle/Frames/enemyIdle.enemyIdle")
        (`NavMovementComponent.StopActiveMovement` (`self.CharacterMovement`))
        (set `self.isIdle` true)
        (`CharacterMovementComponent.SetMovementMode` (`self.CharacterMovement`) "MOVE_NavWalking" 0)
        (`PaperFlipbookComponent.SetFlipbook` (`self.Sprite`) "/Game/Yugen/Assets/Flipbooks/Enemy/EnemyIdle/Frames/enemyIdle.enemyIdle")))))

(fn `Compare Flipbook`
  (params (Flipbook :type "PaperFlipbook Object Reference"))
  (returns (FlipbookAlreadyEnabled :type Boolean))
  (return (== Flipbook (`PaperFlipbookComponent.GetFlipbook` (`self.Sprite`)))))

(fn `Enemy Take Damage`
  (set `self.Enemy Health` (- (`self.Enemy Health`) 1)))

(fn `UserConstructionScript`
  (set `InterpToMovementComponent.ControlPoints` (`|MakeArray` (make `InterpControlPoint` (`self.PointA`)) (make `InterpControlPoint` (`self.PointB`))) (`self.InterpToMovement`)))